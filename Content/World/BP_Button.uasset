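; BP_Button is an interactable world button with a short text label and a press animation.
; Interaction flags it as interacted while the ButtonMovement timeline offsets the mesh's Z from its current position each update, clearing the flag on finish.
; Cursor hover toggles custom depth on the mesh.
; Other events set the widget label, truncated to three characters, and apply a preview material to both material slots.
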(event `self.ReceiveBeginPlay`
  (`PrimitiveComponent.SetCastShadow` (`self.WidgetText`) false))

(event `self.OnInteract`
  (bind _buttonmesh (`self.ButtonMesh`))
  (bind (_relativelocation_x _relativelocation_y _relativelocation_z) (`KismetMathLibrary.BreakVector` (`SceneComponent.RelativeLocation` _buttonmesh)))
  (set `self.bIsInteracted` true)
  (bind (_direction _buttonmovement) (`Timeline|ButtonMovement` :!via `PlayFromStart`)
    (:`Update`
      (`SceneComponent.K2_SetRelativeLocation` _buttonmesh (`KismetMathLibrary.MakeVector` _relativelocation_x _relativelocation_y (+ _relativelocation_z _buttonmovement)) false false))
    (:`Finished`
      (set `self.bIsInteracted` false))))

(event `self.SetButtonText`
  (params (Text :type String))
  (bind _asdp_text_widget (cast `DP_TextWidget` (`WidgetComponent.GetWidget` (`self.WidgetText`))))
  (`DP_TextWidget.SetText` _asdp_text_widget (`KismetTextLibrary.Conv_StringToText` (`KismetStringLibrary.GetSubstring` Text 0 3))))

(event `self.OnBeginCursorHover`
  (params (TouchedActor :type "Actor Object Reference"))
  (`PrimitiveComponent.SetRenderCustomDepth` (`self.ButtonMesh`) true))

(event `self.OnEndCursorHover`
  (params (TouchedActor :type "Actor Object Reference"))
  (`PrimitiveComponent.SetRenderCustomDepth` (`self.ButtonMesh`) false))

(event `self.UpdatePreview`
  (params (PreviewMaterial :type "MaterialInterface Object Reference"))
  (for _index (range 2)
    (`PrimitiveComponent.SetMaterial` (`self.ButtonMesh`) _index PreviewMaterial)))

(fn `UserConstructionScript`)