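; BP_Display_8 is a world display actor with a body, a glass mesh and eight segment meshes; the graph only handles its preview appearance.
; UpdatePreview applies the supplied preview material to three body material slots and the glass, and turns off shadow casting on both.
; It also hides all eight segment meshes, leaving the body and glass as the preview.
; The construction script is empty.
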(event `self.UpdatePreview`
  (params (PreviewMaterial :type "MaterialInterface Object Reference"))
  (bind _bodymesh (`self.BodyMesh`))
  (bind _glassmesh (`self.GlassMesh`))
  (`|ExecutionSequence`
    (:`then_0`
      (for _index (range 3)
        (`PrimitiveComponent.SetMaterial` _bodymesh _index PreviewMaterial))
      (`PrimitiveComponent.SetCastShadow` _bodymesh false))
    (:`then_1`
      (`PrimitiveComponent.SetMaterial` _glassmesh 0 PreviewMaterial)
      (`PrimitiveComponent.SetCastShadow` _glassmesh false))
    (:`then_2`
      (`SceneComponent.SetVisibility` (`self.Mesh Segment 1`) false false)
      (`SceneComponent.SetVisibility` (`self.Mesh Segment 2`) false false)
      (`SceneComponent.SetVisibility` (`self.Mesh Segment 3`) false false)
      (`SceneComponent.SetVisibility` (`self.Mesh Segment 4`) false false)
      (`SceneComponent.SetVisibility` (`self.Mesh Segment 5`) false false)
      (`SceneComponent.SetVisibility` (`self.Mesh Segment 6`) false false)
      (`SceneComponent.SetVisibility` (`self.Mesh Segment 7`) false false)
      (`SceneComponent.SetVisibility` (`self.Mesh Segment 8`) false false))))

(fn `UserConstructionScript`)